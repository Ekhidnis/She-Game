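; Door actor that swings open and closed in response to the OnOpen and OnClose events of its OpenDoor component.
; It stores its starting rotation at BeginPlay, and the OpenDoorAnim timeline adds an animated yaw to that rotation.
; Opening plays the timeline and closing reverses it, while an event track on the timeline triggers the door sound at the actor's location.
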(event `self.ReceiveBeginPlay`
  (set `self.Initial Rotation` (`self.K2_GetActorRotation`)))

(event `self.OpenDoor.OnOpen`
  (bind (_direction _open_door_animation) (`Timeline|Open Door Anim` :!label _label)
    (:`Update`
      (`self.K2_SetActorRotation` (`KismetMathLibrary.ComposeRotators` (`self.Initial Rotation`) (`KismetMathLibrary.MakeRotator` 0.0 0.0 _open_door_animation))))
    (:`Open Door Sound`
      (`GameplayStatics.PlaySoundAtLocation` "/Game/Sounds/OpenDoorSound.OpenDoorSound" (`self.K2_GetActorLocation`) (struct) 1.0 2.0 0.0 null null null))))

(event `self.OpenDoor.OnClose`
  (goto _label :!via `Reverse`))

(fn `UserConstructionScript`)