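; Gate Blueprint for a gate that moves vertically when its OpenGate event is called.
; A DoOnce records the starting location and plays a low-pitched bell, then after a short delay a whoosh plays as movement begins.
; The GateAnimation timeline drives a Z offset from that stored location, moving the whole actor without sweep.
; Nothing in this graph resets the DoOnce or reverses the motion.
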(event `OpenGate`
  (`/Engine/EditorBlueprintResources/StandardMacros.DoOnce` false
    (:`Completed`
      ;[1 1 1] SET DEFAULT LOC
      (bind _output_get (set `self.CastToObjectDefaultLoc` (`SceneComponent.K2_GetComponentLocation` (`self.RootComponent`))))
      (`GameplayStatics.PlaySoundAtLocation` "/Game/Sounds/BellElevatorRing_S08FO_123.BellElevatorRing_S08FO_123" _output_get (struct) 0.5 0.5 0.0 null null null)
      (`KismetSystemLibrary.Delay` 1.5)
      (`GameplayStatics.PlaySoundAtLocation` "/Game/Sounds/large_whoosh_10.large_whoosh_10" _output_get (struct) 1.0 1.0 0.0 null null null)
      ;[1 1 1] MOVE GATE
      (bind (_direction _button_anim) (`Timeline|Gate Animation` :!via `PlayFromStart`)
        (:`Update`
          (`self.K2_SetActorLocation` (+ _output_get (`KismetMathLibrary.MakeVector` 0.0 0.0 _button_anim))))))))

(fn `UserConstructionScript`)