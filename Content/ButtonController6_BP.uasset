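; Controller for the sixth button puzzle, a six-button switching puzzle that drives two gates once ButtonController5 is completed.
; CheckLogic6 identifies the button passed in, calls SwitchButton on three linked buttons and plays that button's ping note.
; It then checks button states: all pressed closes gate 1, opens gate 2 and turns the cube red, while all released does the reverse in green.
; BeginPlay runs the same logic.
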(event `self.ReceiveBeginPlay`
  (bind _button_bp_1_reference (`self.Button_BP 1 Reference`))
  (bind _button_bp_4_reference (`self.Button_BP 4 Reference`))
  (bind _gate_bp_reference (`self.Gate_BP Reference`))
  (bind _gate_bp_2_reference (`self.Gate_BP_2 Reference`))
  (bind _button_bp_2_reference (`self.Button_BP 2 Reference`))
  (bind _button_bp_5_reference (`self.Button_BP 5 Reference`))
  (bind _button_bp_3_reference (`self.Button_BP 3 Reference`))
  (bind _button_bp_6_reference (`self.Button_BP 6 Reference`))
  (bind _ispressed (`/Game/Button_BP.IsPressed` _button_bp_6_reference))
  (bind _ispressed_2 (`/Game/Button_BP.IsPressed` _button_bp_1_reference))
  (bind _ispressed_3 (`/Game/Button_BP.IsPressed` _button_bp_4_reference))
  (bind _ispressed_4 (`/Game/Button_BP.IsPressed` _button_bp_5_reference))
  (bind _ispressed_5 (`/Game/Button_BP.IsPressed` _button_bp_2_reference))
  (bind _ispressed_6 (`/Game/Button_BP.IsPressed` _button_bp_3_reference))
  (if (`/Game/ButtonController5_BP.IsCompleted` (`self.ButtonController5 Reference`)) :!label _label
    ;[1 1 1] SWITCH OTHER BUTTONS LOGIC
    (if (== _button_bp_1_reference (stale `CheckLogic6` NewParam))
      (`/Game/Button_BP.SwitchButton` _button_bp_3_reference false)
      (`/Game/Button_BP.SwitchButton` _button_bp_4_reference false)
      (`/Game/Button_BP.SwitchButton` _button_bp_5_reference false)
      ;[1 1 1] PLAY NOTE SOUND
      (`GameplayStatics.PlaySoundAtLocation` "/Game/Sounds/Ping_A.Ping_A" (`self.K2_GetActorLocation` _button_bp_1_reference) (struct) 0.5 0.5 0.0 null null null)
      (elif (== _button_bp_2_reference (stale `CheckLogic6` NewParam))
        (`/Game/Button_BP.SwitchButton` _button_bp_4_reference false)
        (`/Game/Button_BP.SwitchButton` _button_bp_5_reference false)
        (`/Game/Button_BP.SwitchButton` _button_bp_6_reference false)
        (`GameplayStatics.PlaySoundAtLocation` "/Game/Sounds/Ping_C.Ping_C" (`self.K2_GetActorLocation` _button_bp_2_reference) (struct) 0.5 0.5 0.0 null null null)
        (elif (== _button_bp_3_reference (stale `CheckLogic6` NewParam))
          (`/Game/Button_BP.SwitchButton` _button_bp_1_reference false)
          (`/Game/Button_BP.SwitchButton` _button_bp_6_reference false)
          (`/Game/Button_BP.SwitchButton` _button_bp_5_reference false)
          (`GameplayStatics.PlaySoundAtLocation` "/Game/Sounds/Ping_C6.Ping_C6" (`self.K2_GetActorLocation` _button_bp_3_reference) (struct) 0.5 0.5 0.0 null null null)
          (elif (== _button_bp_4_reference (stale `CheckLogic6` NewParam))
            (`/Game/Button_BP.SwitchButton` _button_bp_2_reference false)
            (`/Game/Button_BP.SwitchButton` _button_bp_1_reference false)
            (`/Game/Button_BP.SwitchButton` _button_bp_6_reference false)
            (`GameplayStatics.PlaySoundAtLocation` "/Game/Sounds/Ping_D_.Ping_D_" (`self.K2_GetActorLocation` _button_bp_4_reference) (struct) 1.0 0.5 0.0 null null null)
            (elif (== _button_bp_5_reference (stale `CheckLogic6` NewParam))
              (`/Game/Button_BP.SwitchButton` _button_bp_3_reference false)
              (`/Game/Button_BP.SwitchButton` _button_bp_2_reference false)
              (`/Game/Button_BP.SwitchButton` _button_bp_1_reference false)
              (`GameplayStatics.PlaySoundAtLocation` "/Game/Sounds/Ping_F_.Ping_F_" (`self.K2_GetActorLocation` _button_bp_5_reference) (struct) 0.3 0.5 0.0 null null null)
              (elif (== _button_bp_6_reference (stale `CheckLogic6` NewParam))
                (`/Game/Button_BP.SwitchButton` _button_bp_4_reference false)
                (`/Game/Button_BP.SwitchButton` _button_bp_3_reference false)
                (`/Game/Button_BP.SwitchButton` _button_bp_2_reference false)
                (`GameplayStatics.PlaySoundAtLocation` "/Game/Sounds/Ping_F_.Ping_F_" (`self.K2_GetActorLocation` _button_bp_6_reference) (struct) 0.3 0.5 0.0 null null null)))))))
    (if (and (and (and (and (and _ispressed_2 _ispressed_5) _ispressed_6) _ispressed_3) _ispressed_4) _ispressed)
      ;[1 1 1] OPEN GATE #1
      (`/Game/Gate_BP.SwitchGate` _gate_bp_reference false true)
      (`PrimitiveComponent.SetMaterial` (`self.Cube`) 0 "/Game/Materials/Red.Red")
      ;[1 1 1] OPEN GATE #2
      (`/Game/Gate_BP.SwitchGate` _gate_bp_2_reference true false)
      (elif (and (and (and (and (and (not _ispressed_2) (not _ispressed_5)) (not _ispressed_6)) (not _ispressed_3)) (not _ispressed_4)) (not _ispressed))
        ;[1 1 1] OPEN GATE #1
        (`/Game/Gate_BP.SwitchGate` _gate_bp_reference true false)
        (`PrimitiveComponent.SetMaterial` (`self.Cube`) 0 "/Game/Materials/Green.Green")
        ;[1 1 1] CLOSE GATE #2
        (`/Game/Gate_BP.SwitchGate` _gate_bp_2_reference false true)))))

(event `CheckLogic6`
  (params (NewParam :type "/Game/Button_BP Object Reference"))
  (goto _label))

(fn `UserConstructionScript`)