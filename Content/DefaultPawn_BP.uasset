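; Player pawn blueprint that adds footstep audio, night ambience and button interaction.
; Each WASD press plays one of five footstep sounds at the camera, picked through chained branches that re-roll the random number, so odds are uneven.
; F runs a short, debug-drawn line trace from the camera and presses any Button_BP it hits.
; BeginPlay starts the 2D Night sound.
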(event `Key|W`
  (params (Key :type "Key Structure"))
  (bind _returnvalue (`KismetMathLibrary.RandomInteger` 5))
  (bind _foot_steps_volume (`self.Foot Steps Volume`))
  (bind _returnvalue_2 (`SceneComponent.K2_GetComponentLocation` (`self.Camera`)))
  ;[1 1 1] PLAY RANDOM FOOT STEP SOUND ON WASD INPUT
  (:`Pressed`
    (if (== _returnvalue 0) :!label _label
      (`GameplayStatics.PlaySoundAtLocation` "/Game/Sounds/Foot_Step__1_.Foot_Step__1_" _returnvalue_2 (struct) _foot_steps_volume 1.0 0.0 null null null)
      (elif (== _returnvalue 1)
        (`GameplayStatics.PlaySoundAtLocation` "/Game/Sounds/Foot_Step__2_.Foot_Step__2_" _returnvalue_2 (struct) _foot_steps_volume 1.0 0.0 null null null)
        (elif (== _returnvalue 2)
          (`GameplayStatics.PlaySoundAtLocation` "/Game/Sounds/Foot_Step__3_.Foot_Step__3_" _returnvalue_2 (struct) _foot_steps_volume 1.0 0.0 null null null)
          (elif (== _returnvalue 3)
            (`GameplayStatics.PlaySoundAtLocation` "/Game/Sounds/Foot_Step__4_.Foot_Step__4_" _returnvalue_2 (struct) _foot_steps_volume 1.0 0.0 null null null)
            (else
              (`GameplayStatics.PlaySoundAtLocation` "/Game/Sounds/Foot_Step__5_.Foot_Step__5_" _returnvalue_2 (struct) _foot_steps_volume 1.0 0.0 null null null))))))))

(event `Key|A`
  (params (Key :type "Key Structure"))
  ;[1 1 1] PLAY RANDOM FOOT STEP SOUND ON WASD INPUT
  (:`Pressed`
    (goto _label)))

(event `Key|S`
  (params (Key :type "Key Structure"))
  ;[1 1 1] PLAY RANDOM FOOT STEP SOUND ON WASD INPUT
  (:`Pressed`
    (goto _label)))

(event `Key|D`
  (params (Key :type "Key Structure"))
  ;[1 1 1] PLAY RANDOM FOOT STEP SOUND ON WASD INPUT
  (:`Pressed`
    (goto _label)))

(event `Key|F`
  (params (Key :type "Key Structure"))
  (bind _camera (`self.Camera`))
  (bind _returnvalue (`SceneComponent.K2_GetComponentLocation` _camera))
  ;[1 1 1] LINE TRACE FROM PAWN VIEWPOINT ON F INPUT
  (:`Pressed`
    (bind _outhit (`KismetSystemLibrary.LineTraceSingle` :`Start` _returnvalue :`End` (+ _returnvalue (* (`SceneComponent.GetForwardVector` _camera) 200.0)) :`TraceChannel` "TraceTypeQuery1" :`bTraceComplex` true :`DrawDebugType` "ForDuration"))
    (bind _asbutton_bp (cast `/Game/Button_BP` (`.HitActor` (`GameplayStatics.BreakHitResult` _outhit))))
    (`/Game/Button_BP.ButtonIsPressed` _asbutton_bp true)))

(event `self.ReceiveBeginPlay`
  (`GameplayStatics.PlaySound2D` "/Game/Sounds/Night.Night" 0.5 1.0 0.0 null null))

(fn `UserConstructionScript`)