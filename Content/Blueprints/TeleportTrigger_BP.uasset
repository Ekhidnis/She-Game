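; Trigger volume that teleports an overlapping DefaultPawn_BP or ActionBlock_BP to the TeleportDest actor's location with zero rotation and plays a sound.
; A pawn's movement component is stopped and deactivated for a one-second delay, then reactivated.
; A DoOnce gate blocks further teleports until the delay ends, resetting at once for other actor types.
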(event `self.CollisionComponent.OnComponentBeginOverlap`
  (params (OverlappedComponent :type "PrimitiveComponent Object Reference") (OtherActor :type "Actor Object Reference") (OtherComp :type "PrimitiveComponent Object Reference") (OtherBodyIndex :type Integer) (bFromSweep :type Boolean) (SweepResult :type "HitResult Structure (by ref)"))
  (bind _returnvalue (`SceneComponent.K2_GetComponentLocation` (`/Game/Blueprints/TeleportDest_BP.DefaultSceneRoot` (`self.TeleportDest`))))
  (`/Engine/EditorBlueprintResources/StandardMacros.DoOnce` false :!label _label
    (:`Completed`
      (bind _asdefault_pawn_bp (cast `/Game/Blueprints/DefaultPawn_BP` OtherActor)
        (:`then`
          (`self.K2_TeleportTo` :`self` _asdefault_pawn_bp :`DestLocation` _returnvalue)
          (bind _movementcomponent (`DefaultPawn.MovementComponent` _asdefault_pawn_bp))
          (`MovementComponent.StopMovementImmediately` _movementcomponent)
          (`ActorComponent.Deactivate` _movementcomponent)
          (`GameplayStatics.PlaySound2D` "/Game/Sounds/TeleportSound.TeleportSound" 1.0 1.0 0.0 null null)
          (`KismetSystemLibrary.Delay` 1.0)
          (`ActorComponent.Activate` _movementcomponent false)
          (`MovementComponent.StopMovementImmediately` _movementcomponent)
          (goto _label :!via `Reset`))
        (:`CastFailed`
          (bind _asaction_block_bp (cast `/Game/Blueprints/Objects_BP/ActionBlock_BP` OtherActor)
            (:`then`
              (`self.K2_TeleportTo` :`self` _asaction_block_bp :`DestLocation` _returnvalue)
              (`GameplayStatics.PlaySound2D` "/Game/Sounds/TeleportSound.TeleportSound" 1.0 1.0 0.0 null null)
              (`KismetSystemLibrary.Delay` 1.0)
              (goto _label :!via `Reset`))
            (:`CastFailed`
              (goto _label :!via `Reset`))))))))

(fn `UserConstructionScript`)