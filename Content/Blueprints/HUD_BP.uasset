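; HUD Blueprint that draws a simple on-screen crosshair and an interaction hint.
; Each DrawHUD event draws a pale yellow square from the screen center, sized by the RectangleSizeActual variable.
; It also draws a white "Press Left Mouse to interact" prompt near the top-left, unconditionally, with both positions derived from the viewport size.
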(event `self.ReceiveDrawHUD`
  (params (SizeX :type Integer) (SizeY :type Integer))
  (bind _rectanglesizeactual (`self.RectangleSizeActual`))
  (`self.DrawRect` (struct :`R` 1.0 :`G` 0.974054 :`B` 0.578125 :`A` 1.0) (`KismetMathLibrary.Conv_IntToDouble` (/ SizeX 2)) (`KismetMathLibrary.Conv_IntToDouble` (/ SizeY 2)) _rectanglesizeactual _rectanglesizeactual)
  (`self.DrawText` "Press \"Left Mouse\" to interact" (struct :`R` 1.0 :`G` 1.0 :`B` 1.0 :`A` 1.0) (`KismetMathLibrary.Conv_IntToDouble` (/ SizeX 32)) (`KismetMathLibrary.Conv_IntToDouble` (/ SizeY 18)) null 3.0))

(fn `UserConstructionScript`)