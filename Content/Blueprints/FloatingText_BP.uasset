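; FloatingText_BP is a trigger actor that shows a floating text message on screen when the player's pawn overlaps it.
; A DoOnce gate limits it to a single showing, with no reset wired in the graph.
; It creates a FloatingTextWidget_BP, passes in its FloatingText variable, plays the widget's FloatingTextAnim, then removes the widget after a short delay.
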(event `self.ReceiveActorBeginOverlap`
  (params (OtherActor :type "Actor Object Reference"))
  (if (== OtherActor (`GameplayStatics.GetPlayerPawn` 0))
    (`/Engine/EditorBlueprintResources/StandardMacros.DoOnce` false
      (:`Completed`
        (bind _returnvalue (`|CreateWidget` "/Game/Blueprints/FloatingTextWidget_BP.FloatingTextWidget_BP_C"))
        (set `/Game/Blueprints/FloatingTextWidget_BP.FloatingText` (`self.FloatingText`) _returnvalue)
        (`UserWidget.AddToViewport` _returnvalue 0)
        (`UserWidget.PlayAnimation` _returnvalue (`/Game/Blueprints/FloatingTextWidget_BP.FloatingTextAnim` _returnvalue) 0.0 1 "Forward" 1.0 false)
        (`KismetSystemLibrary.Delay` 3.0)
        (`Widget.RemoveFromParent` _returnvalue)))))

(fn `UserConstructionScript`)