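; Gate actor that opens and closes by moving vertically from the location it records on BeginPlay.
; SwitchGate passes Open or Close through a DoOnce, playing a bell, then after a delay a whoosh as the GateAnimation timeline plays or reverses.
; The timeline's value drives the Z offset, and its update calls ResetButton to re-arm the DoOnce.
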(event `self.ReceiveBeginPlay`
  ;[1 1 1] SET DEFAULT LOC
  (set `self.DefaultLocation` (`SceneComponent.K2_GetComponentLocation` (`self.RootComponent`))))

(event `ResetButton`
  (bind _defaultlocation (`self.DefaultLocation`))
  (goto _label :!via `Reset`))

(event `SwitchGate`
  (params (Open :type Boolean) (Close :type Boolean))
  (bind _defaultlocation (`self.DefaultLocation`))
  (`/Engine/EditorBlueprintResources/StandardMacros.DoOnce` false :!label _label
    (:`Completed`
      (if Open
        (set `self.IsOpen` true)
        (`GameplayStatics.PlaySoundAtLocation` "/Game/Sounds/BellElevatorRing_S08FO_123.BellElevatorRing_S08FO_123" _defaultlocation (struct) 0.5 0.5 0.0 null null null)
        (`KismetSystemLibrary.Delay` 1.5)
        (`GameplayStatics.PlaySoundAtLocation` "/Game/Sounds/large_whoosh_10.large_whoosh_10" _defaultlocation (struct) 1.0 1.0 0.0 null null null)
        ;[1 1 1] MOVE GATE
        (bind (_direction _button_anim) (`Timeline|Gate Animation` :!label _label_2)
          (:`Update`
            (`self.K2_SetActorLocation` (+ _defaultlocation (`KismetMathLibrary.MakeVector` 0.0 0.0 _button_anim)))
            (`self.ResetButton`)))
        (elif Close
          (set `self.IsOpen` false)
          (`GameplayStatics.PlaySoundAtLocation` "/Game/Sounds/BellElevatorRing_S08FO_123.BellElevatorRing_S08FO_123" _defaultlocation (struct) 0.5 0.5 0.0 null null null)
          (`KismetSystemLibrary.Delay` 1.5)
          (`GameplayStatics.PlaySoundAtLocation` "/Game/Sounds/large_whoosh_10.large_whoosh_10" _defaultlocation (struct) 1.0 1.0 0.0 null null null)
          (goto _label_2 :!via `Reverse`))))))

(fn `UserConstructionScript`)