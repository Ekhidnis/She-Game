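; Pressure panel that the player presses by overlapping its box, toggling three linked action blocks open or closed.
; Each press flip-flops a timeline that moves the panel vertically, guarded by a DoOnce that resets when the animation finishes with a click.
; Player presses also toggle a twin panel, passing false to avoid ping-pong.
; Panels flagged Alternate toggle themselves at BeginPlay, so pairs can start in opposite states.
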(event `self.Box.OnComponentBeginOverlap`
  (params (OverlappedComponent :type "PrimitiveComponent Object Reference") (OtherActor :type "Actor Object Reference") (OtherComp :type "PrimitiveComponent Object Reference") (OtherBodyIndex :type Integer) (bFromSweep :type Boolean) (SweepResult :type "HitResult Structure (by ref)"))
  ;[1 1 1] ACTIVATE WHEN OVERLAP PAWN
  (if (and (`PrimitiveComponent.IsOverlappingActor` (`self.Box`) (`GameplayStatics.GetPlayerPawn` 0)) (not (`self.IsPressed`)))
    (`self.Pressed` true)))

(event `Pressed`
  (params (IsPressedByPlayer :type Boolean))
  (bind _starterlocation (`self.StarterLocation`))
  ;[1 1 1] FLIP FLOP ANIM
  (`/Engine/EditorBlueprintResources/StandardMacros.DoOnce` false :!label _label
    (:`Completed`
      (`/Engine/EditorBlueprintResources/StandardMacros.FlipFlop`
        (:`A`
          (set `self.IsPressed` true)
          (bind (_direction _presspanel_anim) (`Timeline|PressPanel Anim` :!label _label_2)
            (:`Update`
              (`self.K2_SetActorLocation` self (+ _starterlocation (`KismetMathLibrary.MakeVector` 0.0 0.0 _presspanel_anim)) false false))
            (:`Finished`
              (`GameplayStatics.PlaySoundAtLocation` "/Game/Sounds/click_8.click_8" _starterlocation (struct) 0.5 1.0 0.0 null null null)
              (`self.Reset Do Once`)
              (`/Game/Blueprints/Objects_BP/ActionButtonBlock_BP.OpenClose` (`self.ActionButtonBlock Ref 1`))
              (`/Game/Blueprints/Objects_BP/ActionButtonBlock_BP.OpenClose` (`self.ActionButtonBlock Ref 2`))
              (`/Game/Blueprints/Objects_BP/ActionButtonBlock_BP.OpenClose` (`self.ActionButtonBlock Ref 3`))
              ;[1 1 1] ALTERNATE TWIN
              (if IsPressedByPlayer
                (`self.Pressed` (`self.PressPanel Ref`) false)))))
        (:`B`
          (set `self.IsPressed` false)
          (goto _label_2 :!via `Reverse`))))))

(event `Reset Do Once`
  ;[1 1 1] FLIP FLOP ANIM
  (goto _label :!via `Reset`))

(event `self.ReceiveBeginPlay`
  ;[1 1 1] ALTERNATE SELF + SET LOC
  (set `self.StarterLocation` (`self.K2_GetActorLocation`))
  (if (`self.Alternate`)
    (`self.Pressed` false)))

(fn `UserConstructionScript`)