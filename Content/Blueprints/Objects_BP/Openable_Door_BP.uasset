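; Openable door actor that swings open and shut, opening automatically when the referenced AI enters its collision volume and closing when it leaves.
; A timeline drives yaw relative to the rotation saved at BeginPlay, playing forward to open and in reverse to close.
; DoOnce gates prevent repeated opens and limit the door sound until the timeline finishes.
; Doors flagged IsOpenedByMechanism skip the closing animation.
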(event `self.ReceiveBeginPlay`
  (set `self.Initial Rotation` (`self.K2_GetActorRotation`)))

(event `OpenDoor`
  (`/Engine/EditorBlueprintResources/StandardMacros.DoOnce` false :!label _label
    (:`Completed`
      ;[1 1 1] Door Animation
      (bind (_direction _open_door_animation) (`Timeline|Open Door Anim` :!label _label_2)
        (:`Update`
          (`|ExecutionSequence`
            (:`then_0`
              ;[1 1 1] Sound
              (`/Engine/EditorBlueprintResources/StandardMacros.DoOnce` false :!label _label_3
                (:`Completed`
                  (`GameplayStatics.PlaySoundAtLocation` "/Game/Sounds/OpenDoorSound.OpenDoorSound" (`self.K2_GetActorLocation`) (struct) 0.2 1.0 1.0 null null null))))
            (:`then_1`
              (`self.K2_SetActorRotation` (`KismetMathLibrary.ComposeRotators` (`self.Initial Rotation`) (`KismetMathLibrary.MakeRotator` 0.0 0.0 _open_door_animation))))))
        (:`Finished`
          (goto _label_3 :!via `Reset`))))))

(event `CloseDoor`
  (`|ExecutionSequence`
    (:`then_0`
      (if (not (`self.Is Opened by Mechanism`))
        (goto _label_2 :!via `Reverse`)))
    (:`then_1`
      (goto _label :!via `Reset`))))

(event `self.CollisionToCloseDoor.OnComponentBeginOverlap`
  (params (OverlappedComponent :type "PrimitiveComponent Object Reference") (OtherActor :type "Actor Object Reference") (OtherComp :type "PrimitiveComponent Object Reference") (OtherBodyIndex :type Integer) (bFromSweep :type Boolean) (SweepResult :type "HitResult Structure (by ref)"))
  ;[1 1 1] AI Opens Door When Is Near
  (if (== OtherActor (`self.AI_BP Ref`))
    (`self.OpenDoor`)))

(event `self.CollisionToCloseDoor.OnComponentEndOverlap`
  (params (OverlappedComponent :type "PrimitiveComponent Object Reference") (OtherActor :type "Actor Object Reference") (OtherComp :type "PrimitiveComponent Object Reference") (OtherBodyIndex :type Integer))
  ;[1 1 1] AI Opens Door When Is Near
  (if (== OtherActor (`self.AI_BP Ref`))
    (`self.CloseDoor`)))

(fn `UserConstructionScript`)