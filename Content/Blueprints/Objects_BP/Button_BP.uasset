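; Pressable puzzle button actor that toggles between pressed and released, swapping its material to match.
; SwitchButton runs through a DoOnce and FlipFlop, playing or reversing a timeline that slides the actor along world Y from the location saved on press.
; When the timeline finishes, player-triggered switches notify two button controllers (5 and 6) to check their logic, then the DoOnce is reset for the next switch.
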(event `SwitchButton`
  (params (IsPressedByPlayer :type Boolean))
  (`/Engine/EditorBlueprintResources/StandardMacros.DoOnce` false :!label _label
    (:`Completed`
      (`/Engine/EditorBlueprintResources/StandardMacros.FlipFlop`
        (:`A`
          (set `self.IsPressed` true)
          (`PrimitiveComponent.SetMaterial` (`self.Button`) 0 "/Game/Materials/PressedButton.PressedButton")
          ;[1 1 1] SET DEFAULT LOC
          (bind _output_get (set `self.CastToObjectDefaultLoc` (`SceneComponent.K2_GetComponentLocation` (`self.RootComponent`))))
          ;[1 1 1] MOVE BUTTON
          (bind (_direction _button_anim) (`Timeline|Button Animation` :!label _label_2)
            (:`Update`
              (`self.K2_SetActorLocation` (+ _output_get (`KismetMathLibrary.MakeVector` 0.0 _button_anim))))
            (:`Finished`
              (if IsPressedByPlayer
                ;[1 1 1] ButtonController_BP.CheckLogic
                (`/Game/Blueprints/Objects_BP/ButtonController5_BP.CheckLogic5` (`self.ButtonController5_BP Reference`) self)
                ;[1 1 1] ButtonController_BP.CheckLogic
                (`/Game/Blueprints/Objects_BP/ButtonController6_BP.CheckLogic6` (`self.ButtonController6_BP Reference`) self))
              (`self.Reset_Button`)
              (`KismetSystemLibrary.PrintString` "BUTTON OUT"))))
        (:`B`
          (set `self.IsPressed` false)
          (`PrimitiveComponent.SetMaterial` (`self.Button`) 0 "/Game/Materials/NotPressedButton.NotPressedButton")
          (goto _label_2 :!via `Reverse`))))))

(event `Reset_Button`
  (goto _label :!via `Reset`))

(fn `UserConstructionScript`)