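; Medical cabinet ("shkaf") actor that the player can hide inside and leave again.
; The CollisionToEnter overlap enables the cabinet's input and opens a gate for the player pawn, reversing both on exit.
; Left click through the gate plays the open animation and calls ToggleHide.
; ToggleHide flips the pawn's visibility and input, blending the camera between player and cabinet; a HideInside event also calls it.
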(event `self.ReceiveBeginPlay`
  (set `self.Player Ref` (`GameplayStatics.GetPlayerPawn` 0)))

(event `Hide Inside`
  (`/Engine/EditorBlueprintResources/StandardMacros.Gate` true
    (:`Exit`
      (`self.ToggleHide`))))

(event `Key|LeftMouseButton`
  (params (Key :type "Key Structure"))
  (:`Pressed`
    (`/Engine/EditorBlueprintResources/StandardMacros.Gate` true :!label _label
      (:`Exit`
        (`|ExecutionSequence`
          (:`then_0`
            (`SkeletalMeshComponent.PlayAnimation` (`self.SkeletalMesh`) "/Game/ImportedObjects/MedicalShkaf/MedicalShkaf_Anim_MedicalShkaf_Open.MedicalShkaf_Anim_MedicalShkaf_Open" false))
          (:`then_1`
            (`self.ToggleHide`)
            (`self.EnableInput` (`GameplayStatics.GetPlayerController` 0) :!label _label_2)
            (goto _label :!via `Open`)))))))

(event `self.CollisionToEnter.OnComponentBeginOverlap`
  (params (OverlappedComponent :type "PrimitiveComponent Object Reference") (OtherActor :type "Actor Object Reference") (OtherComp :type "PrimitiveComponent Object Reference") (OtherBodyIndex :type Integer) (bFromSweep :type Boolean) (SweepResult :type "HitResult Structure (by ref)"))
  (if (== OtherActor (`GameplayStatics.GetPlayerPawn` 0))
    (cast `/Game/Blueprints/DefaultPawn_BP` OtherActor)
    (goto _label_2)))

(event `self.CollisionToEnter.OnComponentEndOverlap`
  (params (OverlappedComponent :type "PrimitiveComponent Object Reference") (OtherActor :type "Actor Object Reference") (OtherComp :type "PrimitiveComponent Object Reference") (OtherBodyIndex :type Integer))
  (if (== OtherActor (`GameplayStatics.GetPlayerPawn` 0))
    (cast `/Game/Blueprints/DefaultPawn_BP` OtherActor)
    (`self.DisableInput` (`GameplayStatics.GetPlayerController` 0))
    (goto _label :!via `Close`)))

(fn `ToggleHide`
  (bind _returnvalue (`GameplayStatics.GetPlayerController` 0))
  (bind _player_ref (`self.Player Ref`))
  (if (`self.IsHiding`)
    (set `self.IsHiding` false)
    (`self.SetActorHiddenInGame` _player_ref false)
    (`PlayerController.SetViewTargetWithBlend` _returnvalue _player_ref 0.6 "VTBlend_Linear" 0.0 false)
    (`self.EnableInput` _player_ref _returnvalue)
    (else
      (set `self.IsHiding` true)
      (`self.SetActorHiddenInGame` _player_ref true)
      (`PlayerController.SetViewTargetWithBlend` _returnvalue self 0.6 "VTBlend_Linear" 0.0 false)
      (`self.DisableInput` _player_ref _returnvalue))))

(fn `UserConstructionScript`)