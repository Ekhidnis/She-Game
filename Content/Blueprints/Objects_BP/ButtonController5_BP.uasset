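; Controller for a five-button puzzle that opens a gate once every button is pressed.
; CheckLogic5 identifies the triggering button, calls SwitchButton on two linked buttons and plays that button's note at its location.
; It then checks all five pressed states and marks the puzzle completed when all are on.
; A DoOnce then opens the gate, turns the Cube glowing green and switches a button referenced from Puzzle 2.
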(event `CheckLogic5`
  (params (NewParam :type "/Game/Blueprints/Objects_BP/Button_BP Object Reference"))
  (bind _button_bp_1_reference (`self.Button_BP 1 Reference`))
  (bind _button_bp_4_reference (`self.Button_BP 4 Reference`))
  (bind _button_bp_5_reference (`self.Button_BP 5 Reference`))
  (bind _button_bp_2_reference (`self.Button_BP 2 Reference`))
  (bind _button_bp_3_reference (`self.Button_BP 3 Reference`))
  ;[1 1 1] SWITCH OTHER BUTTONS LOGIC
  (if (== _button_bp_1_reference NewParam)
    (`/Game/Blueprints/Objects_BP/Button_BP.SwitchButton` _button_bp_3_reference false)
    (`/Game/Blueprints/Objects_BP/Button_BP.SwitchButton` _button_bp_4_reference false)
    ;[1 1 1] PLAY NOTE SOUND
    (`GameplayStatics.PlaySoundAtLocation` "/Game/Sounds/Ping_A.Ping_A" (`self.K2_GetActorLocation` _button_bp_1_reference) (struct) 0.5 0.5 0.0 null null null)
    (elif (== _button_bp_2_reference NewParam)
      (`/Game/Blueprints/Objects_BP/Button_BP.SwitchButton` _button_bp_4_reference false)
      (`/Game/Blueprints/Objects_BP/Button_BP.SwitchButton` _button_bp_5_reference false)
      (`GameplayStatics.PlaySoundAtLocation` "/Game/Sounds/Ping_C.Ping_C" (`self.K2_GetActorLocation` _button_bp_2_reference) (struct) 0.5 0.5 0.0 null null null)
      (elif (== _button_bp_3_reference NewParam)
        (`/Game/Blueprints/Objects_BP/Button_BP.SwitchButton` _button_bp_1_reference false)
        (`/Game/Blueprints/Objects_BP/Button_BP.SwitchButton` _button_bp_5_reference false)
        (`GameplayStatics.PlaySoundAtLocation` "/Game/Sounds/Ping_C6.Ping_C6" (`self.K2_GetActorLocation` _button_bp_3_reference) (struct) 0.5 0.5 0.0 null null null)
        (elif (== _button_bp_4_reference NewParam)
          (`/Game/Blueprints/Objects_BP/Button_BP.SwitchButton` _button_bp_1_reference false)
          (`/Game/Blueprints/Objects_BP/Button_BP.SwitchButton` _button_bp_2_reference false)
          (`GameplayStatics.PlaySoundAtLocation` "/Game/Sounds/Ping_D_.Ping_D_" (`self.K2_GetActorLocation` _button_bp_4_reference) (struct) 1.0 0.5 0.0 null null null)
          (elif (== _button_bp_5_reference NewParam)
            (`/Game/Blueprints/Objects_BP/Button_BP.SwitchButton` _button_bp_3_reference false)
            (`/Game/Blueprints/Objects_BP/Button_BP.SwitchButton` _button_bp_2_reference false)
            (`GameplayStatics.PlaySoundAtLocation` "/Game/Sounds/Ping_F_.Ping_F_" (`self.K2_GetActorLocation` _button_bp_5_reference) (struct) 0.3 0.5 0.0 null null null))))))
  (if (and (and (and (and (`/Game/Blueprints/Objects_BP/Button_BP.IsPressed` _button_bp_1_reference) (`/Game/Blueprints/Objects_BP/Button_BP.IsPressed` _button_bp_2_reference)) (`/Game/Blueprints/Objects_BP/Button_BP.IsPressed` _button_bp_3_reference)) (`/Game/Blueprints/Objects_BP/Button_BP.IsPressed` _button_bp_4_reference)) (`/Game/Blueprints/Objects_BP/Button_BP.IsPressed` _button_bp_5_reference))
    (set `self.IsCompleted` true)
    (`/Engine/EditorBlueprintResources/StandardMacros.DoOnce` false
      (:`Completed`
        ;[1 1 1] OPEN GATE
        (`/Game/Blueprints/Objects_BP/Gate_BP.SwitchGate` (`self.Gate_BP Reference`) true false)
        (`PrimitiveComponent.SetMaterial` (`self.Cube`) 0 "/Game/Materials/GlowingGreen.GlowingGreen")
        (`/Game/Blueprints/Objects_BP/Button_BP.SwitchButton` (`self.Button From Puzzle 2 Ref`) true)))))

(fn `UserConstructionScript`)