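; DoorTriggerVolume_BP is a trigger volume that opens a linked Openable_Door_BP while an ActionBlock_BP overlaps it.
; Any overlap sets it active and plays a click, and the first also starts the referenced AI's patrol.
; When the block leaves, the door closes unless an optional secondary trigger is still active.
; An unset secondary reference defaults to itself, so one volume works alone.
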(event `self.CollisionComponent.OnComponentBeginOverlap`
  (params (OverlappedComponent :type "PrimitiveComponent Object Reference") (OtherActor :type "Actor Object Reference") (OtherComp :type "PrimitiveComponent Object Reference") (OtherBodyIndex :type Integer) (bFromSweep :type Boolean) (SweepResult :type "HitResult Structure (by ref)"))
  ;[1 1 1] OPEN CLOSE DOOR
  (`|ExecutionSequence`
    (:`then_0`
      (set `self.IsActive` true)
      (`GameplayStatics.PlaySoundAtLocation` "/Game/Sounds/click_8.click_8" (`self.K2_GetActorLocation` self) (struct) 0.2 0.2 0.06 null null null)
      (if (== (`GameplayStatics.GetObjectClass` OtherActor) "/Game/Blueprints/Objects_BP/ActionBlock_BP.ActionBlock_BP_C")
        (bind _asopenable_door_bp (cast `/Game/Blueprints/Objects_BP/Openable_Door_BP` (`self.OpenableDoor Ref`)))
        (`|ExecutionSequence`
          (:`then_0`
            (set `/Game/Blueprints/Objects_BP/Openable_Door_BP.Is Opened by Mechanism` true _asopenable_door_bp))
          (:`then_1`
            (`/Game/Blueprints/Objects_BP/Openable_Door_BP.OpenDoor` _asopenable_door_bp)))))
    (:`then_1`
      (`/Engine/EditorBlueprintResources/StandardMacros.DoOnce` false
        (:`Completed`
          (`/Game/Blueprints/AI_BP.Patrol` (`self.AI ref`)))))))

(event `self.CollisionComponent.OnComponentEndOverlap`
  (params (OverlappedComponent :type "PrimitiveComponent Object Reference") (OtherActor :type "Actor Object Reference") (OtherComp :type "PrimitiveComponent Object Reference") (OtherBodyIndex :type Integer))
  ;[1 1 1] OPEN CLOSE DOOR
  (set `self.IsActive` false)
  (if (or (`self.IsActive`) (`/Game/Blueprints/Objects_BP/DoorTriggerVolume_BP.IsActive` (`self.Secondary Trigger Ref `)))
    _
    (elif (== (`GameplayStatics.GetObjectClass` OtherActor) "/Game/Blueprints/Objects_BP/ActionBlock_BP.ActionBlock_BP_C")
      (bind _asopenable_door_bp (cast `/Game/Blueprints/Objects_BP/Openable_Door_BP` (`self.OpenableDoor Ref`)))
      (`|ExecutionSequence`
        (:`then_0`
          (set `/Game/Blueprints/Objects_BP/Openable_Door_BP.Is Opened by Mechanism` false _asopenable_door_bp))
        (:`then_1`
          (`/Game/Blueprints/Objects_BP/Openable_Door_BP.CloseDoor` _asopenable_door_bp))))))

(event `self.ReceiveBeginPlay`
  ;[1 1 1] if  ref null set self
  (if (not (`KismetSystemLibrary.IsValid` (`self.Secondary Trigger Ref `)))
    (set `self.Secondary Trigger Ref ` self)))

(fn `UserConstructionScript`)