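; AI_BP is a ghost enemy that patrols, chases the player on sight, and opens the Lose level when its capsule touches them.
; Patrol idles, then moves to one of five random locations, repeating on success.
; PawnSensing starts the chase and heartbeat sound; a one-second retriggerable delay ends it and resumes patrol.
; Cross-resetting DoOnce gates keep standing and flying animation transitions from replaying.
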(event `Patrol`
  ;[1 1 1] PATROL
  (if (not (`self.IsSeeingEnemy`))
    (`self.StateStanding`)
    (`KismetSystemLibrary.Delay` (`KismetMathLibrary.RandomFloatInRange` 1.0 5.0))
    (`|AIMoveTo` self (`KismetArrayLibrary.Array_Random` (`|MakeArray` (`self.Location 1`) (`self.Location 2`) (`self.Location 3`) (`self.Location 4`) (`self.Location 5`))) null 1.0
      (:`then`
        (`self.StateFlying`))
      (:`OnSuccess`
        (`self.Patrol`)))))

(event `StateStanding`
  (bind _mesh (`self.Mesh`))
  (bind _mesh_2 (`self.Mesh`))
  ;[1 1 1] States
  (`/Engine/EditorBlueprintResources/StandardMacros.DoOnce` false :!label _label
    (:`Completed`
      (`SkeletalMeshComponent.PlayAnimation` _mesh_2 "/Game/ImportedObjects/Ghost_Textures/Ghost_Anim_GhostArmature_Ghost_State_FlyingToStanding.Ghost_Anim_GhostArmature_Ghost_State_FlyingToStanding" false)
      (`KismetSystemLibrary.Delay` 0.4)
      (`SkeletalMeshComponent.PlayAnimation` _mesh_2 "/Game/ImportedObjects/Ghost_Textures/Ghost_Anim_GhostArmature_Ghost_State_Standing.Ghost_Anim_GhostArmature_Ghost_State_Standing" true)
      (goto _label_3 :!via `Reset`))))

(event `self.PawnSensing.OnSeePawn`
  (params (Pawn :type "Pawn Object Reference"))
  ;[1 1 1] Chases if sees pawn
  (bind _asdefault_pawn_bp (cast `/Game/Blueprints/DefaultPawn_BP` Pawn))
  (`|ExecutionSequence`
    (:`then_0`
      (set `self.IsSeeingEnemy` true)
      (`self.PlayChaseSound`)
      (`|AIMoveTo` self (0.0 0.0 0.0) _asdefault_pawn_bp
        (:`then`
          (`self.StateFlying`))))
    (:`then_1`
      (`KismetSystemLibrary.RetriggerableDelay` 1.0)
      (set `self.IsSeeingEnemy` false)
      (`self.ResetPlayChaseSOund`)
      (`self.Patrol` :!label _label_2))))

(event `self.ReceiveBeginPlay`
  ;[1 1 1] Chases if sees pawn
  (goto _label_2))

(event `StateFlying`
  (bind _mesh (`self.Mesh`))
  ;[1 1 1] States
  (`/Engine/EditorBlueprintResources/StandardMacros.DoOnce` false :!label _label_3
    (:`Completed`
      (`SkeletalMeshComponent.PlayAnimation` _mesh "/Game/ImportedObjects/Ghost_Textures/Ghost_Anim_GhostArmature_Ghost_State_StandingToFlying.Ghost_Anim_GhostArmature_Ghost_State_StandingToFlying" false)
      (`KismetSystemLibrary.Delay` 0.4)
      (`SkeletalMeshComponent.PlayAnimation` _mesh "/Game/ImportedObjects/Ghost_Textures/Ghost_Anim_GhostArmature_Ghost_State_Flying.Ghost_Anim_GhostArmature_Ghost_State_Flying" true)
      (goto _label :!via `Reset`))))

(event `PlayChaseSound`
  ;[1 1 1] Play Chase Sound
  (`/Engine/EditorBlueprintResources/StandardMacros.DoOnce` false :!label _label_4
    (:`Completed`
      (bind _returnvalue (`GameplayStatics.SpawnSoundAttached` "/Game/Sounds/heartbeat-04.heartbeat-04" (`self.Mesh`) "None" (`self.K2_GetActorLocation`) (struct) "SnapToTargetIncludingScale" false 1.0 1.0 0.0 null null))
      (set `self.Heartbeat` _returnvalue))))

(event `self.CapsuleComponent.OnComponentBeginOverlap`
  (params (OverlappedComponent :type "PrimitiveComponent Object Reference") (OtherActor :type "Actor Object Reference") (OtherComp :type "PrimitiveComponent Object Reference") (OtherBodyIndex :type Integer) (bFromSweep :type Boolean) (SweepResult :type "HitResult Structure (by ref)"))
  ;[1 1 1] LoseOnTouch
  (if (== OtherActor (`GameplayStatics.GetPlayerPawn` 0))
    (`GameplayStatics.OpenLevel` "Lose")))

(event `ResetPlayChaseSOund`
  ;[1 1 1] Play Chase Sound
  (`AudioComponent.Stop` (`self.Heartbeat`))
  (goto _label_4 :!via `Reset`))

(fn `UserConstructionScript`)